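; BP_pawn is a player-controlled pawn with basic movement, look and debug printing, apparently an Unreal starter exercise.
; Axis inputs offset the actor along its forward and right vectors without sweep or delta-time scaling.
; Look axes feed controller rotation, with lookup driving yaw and lookRight driving pitch.
; Tick feeds ShowTimeSet, which accumulates time and prints the seconds modulo sixty whenever that changes; BeginPlay and key presses also print.
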(event EventBeginPlay
  (Development|PrintString "BeginPlay"))

(event EventTick
  (params (DeltaSeconds :type Float%20%28single-precision%29))
  ;[1 1 1] Tick
  (CallFunction|ShowTimeSet DeltaSeconds))

(event Input|ActionEvents|InputActionEnterInput
  (params (Key :type Key%20Structure :default "None"))
  (:Pressed
    (Development|PrintString "enter_pressed")))

(event Input|AxisEvents|InputAxislookup
  (params (AxisValue :type Float%20%28single-precision%29))
  (Pawn|Input|AddControllerYawInput AxisValue))

(event Input|AxisEvents|InputAxislookRight
  (params (AxisValue :type Float%20%28single-precision%29))
  (Pawn|Input|AddControllerPitchInput AxisValue))

(event Input|AxisEvents|InputAxismoveRight
  (params (AxisValue :type Float%20%28single-precision%29))
  ;[1 1 1] 옆 움직임
  (Transformation|AddActorWorldOffset (* (Transformation|GetActorRightVector) (* AxisValue 1e+01))))

(event Input|AxisEvents|InputAxismoveForward
  (params (AxisValue :type Float%20%28single-precision%29))
  ;[0.224 0.4235 1] 앞 움직임
  (Transformation|AddActorWorldOffset (* (Transformation|GetActorForwardVector) (* AxisValue 1e+01))))

(event Input|KeyboardEvents|W
  (params (Key :type Key%20Structure :default "None"))
  (:Pressed
    (Development|PrintString "W_pressed")))

(fn ConstructionScript)

(fn ShowTimeSet
  (params (DeltaSeconds :type Float%20%28single-precision%29))
  (bind _output_get (Variables|Default|SetTotalDeltaSecond (+ DeltaSeconds (Variables|Default|GetTotalDeltaSecond))))
  (if (not (== (Variables|Default|GetBeforeInt) (Math|Float|Floor (Math|Float|%(Float) _output_get 6e+01))))
    (Development|PrintString (Utilities|String|Append "TotalDeltaSecond" (Utilities|String|ToString(Integer) (Math|Float|Floor (Math|Float|%(Float) _output_get 6e+01)))))
    (Variables|Default|SetBeforeInt (Math|Float|Floor (Math|Float|%(Float) _output_get 6e+01)))))