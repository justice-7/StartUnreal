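; BP_MoveLeftRight is an actor that moves its Sphere component around a square loop in relative space, along both X and Y despite the name.
; Tick switches on the integer NewVar0 as a four-state machine, stepping +X, +Y, -X, then -Y at Speed scaled by DeltaSeconds.
; Each leg changes state when the relative location passes its 0 or 100 limit, with no clamping.
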(event EventBeginPlay)

(event Collision|EventActorBeginOverlap
  (params (OtherActor :type Actor%20Object%20Reference)))

(event EventTick
  (params (DeltaSeconds :type Float%20%28single-precision%29))
  (bind _sphere (Variables|Default|GetSphere))
  (bind _speed (Variables|Default|Getspeed))
  (bind _returnvalue (* DeltaSeconds _speed))
  (switch int (Variables|Default|GetNewVar_0)
    (:Default
      ;[1 1 1] 오
      (Transformation|AddRelativeLocation _sphere (Math|Vector|MakeVector _returnvalue 0.0 0.0) false false :!label _label)
      (if (> (.x (Variables|/Script/Engine.SceneComponent|GetRelativeLocation _sphere)) 1e+02)
        (Variables|Default|SetNewVar_0 2)))
    (:0
      (goto _label))
    (:1
      ;[1 1 1] 왼
      (bind _result (Math|Float|NegateFloat _returnvalue)
        (:%20%20
          (Transformation|AddRelativeLocation _sphere (Math|Vector|MakeVector _result 0.0 0.0) false false)
          (if (<= (.x (Variables|/Script/Engine.SceneComponent|GetRelativeLocation _sphere)) 0.0)
            (Variables|Default|SetNewVar_0 3)))))
    (:2
      ;[1 1 1] 아래
      (Transformation|AddRelativeLocation _sphere (Math|Vector|MakeVector 0.0 _returnvalue 0.0) false false)
      (if (> (.y (Variables|/Script/Engine.SceneComponent|GetRelativeLocation _sphere)) 1e+02)
        (Variables|Default|SetNewVar_0 1)))
    (:3
      ;[1 1 1] 위
      (bind _result_2 (Math|Float|NegateFloat _returnvalue)
        (:%20%20
          (Transformation|AddRelativeLocation _sphere (Math|Vector|MakeVector 0.0 _result_2 0.0) false false)
          (if (<= (.y (Variables|/Script/Engine.SceneComponent|GetRelativeLocation _sphere)) 0.0)
            (Variables|Default|SetNewVar_0 0)))))))

(fn ConstructionScript)